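; BP_MenuController is a player controller for the game's menu, putting the UI_Menu widget on screen when play begins.
; A GetUI_Menu helper lazily creates the widget, adds it to the viewport and caches it in Menu, reusing that instance while it stays valid.
; BeginPlay calls the helper, then shows the mouse cursor and switches to UI-only input without locking the mouse.
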(event EventBeginPlay
  (Utilities|GetUIMenu
    (:out
      (Variables|Default|SetbShowMouseCursor true)
      (Input|SetInputModeUIOnly self 0 "DoNotLock"))))

(event EventTick
  (params (DeltaSeconds :type Float%20%28single-precision%29)))

(fn ConstructionScript)