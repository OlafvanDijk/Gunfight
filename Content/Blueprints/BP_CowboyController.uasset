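; Player controller for a networked cowboy shooter, handling aim, shoot and reload input plus round and session flow.
; Client events drive lazily created overlay and animation widgets for ready/go, score and win/lose, and toggle CanShoot, which gates aiming and firing.
; A timeline applies decaying random recoil, reused to scatter aim on new rounds.
; Leaving as host notifies GameState before returning to Level_0 and destroying the session; ClampControllerRotation is empty.
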(event Custom|ClientShowReady
  ;[1 1 1] Show Ready Animation
  (bind _ui (Utilities|GetUIAnimations)
    (:Out
      (Default|ShowReady _ui))))

(event Custom|ClientEnableInput
  ;[1 1 1] Show Go Animation, Flash Recticle, Enable Input
  (Utilities|FlowControl|Sequence
    (:then_0
      (bind _ui (Utilities|GetUIAnimations)
        (:Out
          (Default|ShowGo _ui)
          (Default|FlashReticle _ui))))
    (:then_1
      (Variables|Default|SetcanShoot true)
      (bind _asbp_cowboy_character (Utilities|GetPawn)
        (:then
          (bind _ui_2 (Utilities|GetUIOverlay)
            (:Out
              (Default|SetUI _asbp_cowboy_character _ui_2)
              (Default|LocalStartAiming _asbp_cowboy_character))))))))

(event Custom|SetCursorToRandomPos
  (bind (_recoilx _recoily) (Utilities|GetRecoil))
  (bind (_x _y) (Utilities|GetRecoilBeginRound _recoilx _recoily))
  ;[1 1 1] Set Cursor to a random position when a new round has been started
  (CallFunction|MouseRecoil _x _y))

(event Custom|LeaveSession
  ;[1 1 1] Leave Session. If host first throw out the other players.
  (Networking|SwitchHasAuthority
    (:Authority
      (bind _asbp_shooter_game_state (Utilities|Casting|CastToBP_ShooterGameState (Game|GetGameState)))
      (Default|PlayerLeft _asbp_shooter_game_state self)
      (Utilities|FlowControl|Delay 1.0))
    (:Remote
      _))
  (Game|OpenLevel(byName) "Level_0")
  (|DestroySession self))

(event Custom|ClampControllerRotation)

(event Custom|PossessPawn
  (params (CowboyCharater :type BP%20Cowboy%20Character%20Object%20Reference))
  ;[1 1 1] Posses Pawn (Take control)
  (Pawn|Possess CowboyCharater))

(event Custom|ClientSetNewScore
  (params (My%20score :type Integer) (Enemy%20score :type Integer))
  ;[1 1 1] Set New Score
  (bind _ui (Utilities|GetUIOverlay)
    (:Out
      (Default|UpdateLabel _ui My%20score Enemy%20score))))

(event Custom|SetBulletsUI
  (params (Bullets :type Integer))
  (bind _ui_overlay (Variables|Default|GetUI_Overlay))
  ;[1 1 1] Set Bullets amount in the UI
  (Utilities|IsValid _ui_overlay
    (:Is%20Valid
      (Default|SetBulletsEvent _ui_overlay Bullets))))

(event Custom|ClientDisableShooting
  ;[1 1 1] Disable Shooting
  (Variables|Default|SetcanShoot false))

(event Custom|MouseRecoil
  (params (RecoilX :type Float%20%28single-precision%29) (RecoilY :type Float%20%28single-precision%29))
  ;[1 1 1] Mouse Recoil
  (bind _alpha (Timeline|RecoilTimeLine PlayFromStart)
    (:Update
      (Class|PlayerController|AddYawInput (.Yaw (Utilities|GetPitchandYawRecoil RecoilX RecoilY _alpha)))
      (Class|PlayerController|AddPitchInput (.Pitch (Utilities|GetPitchandYawRecoil RecoilX RecoilY _alpha))))))

(event Custom|ShowWinOrLose
  (params (Win :type Boolean))
  ;[1 1 1] Show Win or Lose Animation
  (bind _ui (Utilities|GetUIAnimations)
    (:Out
      (if Win
        (Default|ShowWin _ui)
        (else
          (Default|ShowLose _ui))))))

(event Custom|EnableInputUI
  ;[1 1 1] Enables Input for UI Only
  (Input|SetInputModeUIOnly self 0 "DoNotLock")
  (Variables|Default|SetbShowMouseCursor true))

(event EventBeginPlay
  (Input|SetInputModeGameOnly self))

(event EventTick
  (params (DeltaSeconds :type Float%20%28single-precision%29)))

(event Input|ActionEvents|InputActionShoot
  (params (Key :type Key%20Structure :default "None"))
  (bind (_recoilx _recoily) (Utilities|GetRecoil))
  ;[1 1 1] Shoot Action. If Allowed To Aim and Has Bullets
  (:Pressed
    (Utilities|AllowedtoAim
      (:true
        (Utilities|FlowControl|Sequence
          (:then_0
            (Utilities|HasBullets
              (:Out
                (bind _ui (Utilities|GetUIAnimations)
                  (:Out
                    (Default|FlashReticle _ui)
                    (Class|PlayerController|ClientPlayCameraShake "/Game/Blueprints/CamShake_01.CamShake_01_C" 1.0 "CameraLocal" "0, 0, 0")
                    (CallFunction|MouseRecoil _recoilx _recoily))))))
          (:then_1
            (bind _asbp_cowboy_character (Utilities|GetPawn)
              (:then
                (Default|FireWeapon _asbp_cowboy_character)))))))))

(event Input|ActionEvents|InputActionReload
  (params (Key :type Key%20Structure :default "None"))
  ;[1 1 1] Reload Action Bind
  (:Pressed
    (bind _asbp_cowboy_character (Utilities|GetPawn)
      (:then
        (Default|Reload _asbp_cowboy_character)))))

(event Input|AxisEvents|InputAxisLookRight
  (params (AxisValue :type Float%20%28single-precision%29))
  ;[1 1 1] Change Left + Right Rotation If Allowed To Aim
  (Utilities|AllowedtoAim
    (:true
      (Class|PlayerController|AddYawInput AxisValue)
      (CallFunction|ClampControllerRotation))))

(event Input|AxisEvents|InputAxisLookDown
  (params (AxisValue :type Float%20%28single-precision%29))
  ;[1 1 1] Change Up + Down Rotation If Allowed To Aim
  (Utilities|AllowedtoAim
    (:true
      (Class|PlayerController|AddPitchInput AxisValue)
      (CallFunction|ClampControllerRotation))))

(fn ConstructionScript)