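; Cowboy character Blueprint for revolver play: aiming zoom via FOV timeline, unholstering by swapping hip and hand meshes, and firing.
; Firing traces from the camera, then from the barrel toward that point, to find the hit cowboy and bone.
; ServerFireWeapon applies damage, higher on weak-spot bones, then MulticastFireWeapon plays recoil, projectile and camera shake.
; Zero-health handling is empty, and debug prints and trace drawing remain.
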(event Custom|LocalStartAiming
  (bind _alpha (Timeline|IncreaseFOVTimeline PlayFromStart)
    (:Update
      (Camera|SetFieldOfView (Variables|Default|GetCamera) (Math|Float|Lerp 9e+01 7e+01 _alpha)))))

(event Custom|ReceiveDamage
  (params (BoneName :type Name))
  (bind _weakspots (Variables|Default|GetWeakSpots))
  (bind _returnvalue (Utilities|Array|ContainsItem _weakspots BoneName))
  (bind _returnvalue_2 (Math|Float|SelectFloat 1e+02 25.0 _returnvalue))
  (Development|PrintString (Utilities|String|ToString(Float) _returnvalue_2))
  (Variables|Default|SetHealth (- (Variables|Default|GetHealth) _returnvalue_2))
  (if (<= (Variables|Default|GetHealth) 0.0)
    _))

(event Custom|UnholsterWeapon
  (Variables|Default|SetAiming true)
  (Development|SetHiddeninGame (Variables|Default|GetRevolver_Hip) true false)
  (Development|SetHiddeninGame (Variables|Default|GetRevolver_Hand) false false))

(event Custom|FireWeapon
  (bind _impactpoint (CallFunction|DetermineLookLocation))
  (bind (_locationendhit _physmat _hitbonename _enemyhit) (CallFunction|DetermineBulletLocation _impactpoint))
  (CallFunction|ServerFireWeapon _locationendhit _physmat _hitbonename _enemyhit))

(event Custom|MulticastFireWeapon
  (params (LocationEndHit :type Vector) (Phys%20Mat :type Physical%20Material%20Object%20Reference))
  (bind _mesh (Variables|Character|GetMesh))
  (bind _revolver_hand (Variables|Default|GetRevolver_Hand))
  (bind _returnvalue (Components|SkeletalMesh|GetAnimInstance _mesh))
  (bind _returnvalue_2 (Transformation|GetSocketTransform _revolver_hand "Barrel" "RTS_World"))
  (Animation|Montage|MontageStop _returnvalue 0.0 0)
  (Animation|Montage|MontagePlay _returnvalue "/Game/Animations/MONT_Cowboy_Recoil.MONT_Cowboy_Recoil" 1.0 "MontageLength" 0.0 true)
  (Game|SpawnActorfromClass "/Game/Blueprints/BP_Projectile.BP_Projectile_C" (Math|Transform|MakeTransform (.location _returnvalue_2) (Math|Rotator|FindLookatRotation (.location _returnvalue_2) LocationEndHit) "1,1,1") "AlwaysSpawn" 0 0)
  (Camera|PlayWorldCameraShake "/Game/Blueprints/CamShake_01.CamShake_01_C" (.location _returnvalue_2) 0.0 5e+02))

(event Custom|ServerFireWeapon
  (params (LocationEndHit :type Vector) (Phys%20Mat :type Physical%20Material%20Object%20Reference) (HitBoneName :type Name) (EnemyHit :type BP%20Cowboy%20Character%20Object%20Reference))
  (Utilities|FlowControl|Sequence
    (:then_0
      (Utilities|IsValid EnemyHit
        (:Is%20Valid
          (CallFunction|ReceiveDamage EnemyHit HitBoneName))))
    (:then_1
      (CallFunction|MulticastFireWeapon LocationEndHit Phys%20Mat))))

(event EventBeginPlay)

(fn ConstructionScript)

(fn DetermineLookLocation
  (bind _camera (Variables|Default|GetCamera))
  (bind _maxdistance (LocalVariables|GetMaxDistance))
  (bind _returnvalue (Transformation|GetWorldRotation _camera))
  (bind _returnvalue_2 (Transformation|GetWorldLocation _camera))
  (bind _returnvalue_3 (Math|Vector|GetForwardVector _returnvalue))
  (bind _returnvalue_4 (* _returnvalue_3 _maxdistance))
  (bind _returnvalue_5 (+ _returnvalue_4 _returnvalue_2))
  (bind (_outhit _returnvalue_6) (Collision|LineTraceByChannel _returnvalue_2 _returnvalue_5 "TraceTypeQuery3" false 0 "None"))
  (if _returnvalue_6
    (return (.ImpactPoint (Collision|BreakHitResult _outhit)))
    (else
      (return _returnvalue_5))))

(fn DetermineBulletLocation
  (params (LocationEnd :type Vector))
  (bind (_outhit _returnvalue) (Collision|LineTraceByChannel (Transformation|GetSocketLocation (Variables|Default|GetRevolver_Hand) "Barrel") LocationEnd "TraceTypeQuery3" false 0 "ForDuration"))
  (if _returnvalue
    (bind _asbp_cowboy_character (Utilities|Casting|CastToBP_CowboyCharacter (.HitActor (Collision|BreakHitResult _outhit)))
      (:then
        (Development|PrintString (Utilities|String|ToString(Name) (.HitBoneName (Collision|BreakHitResult _outhit))))
        (return (.ImpactPoint (Collision|BreakHitResult _outhit)) (.PhysMat (Collision|BreakHitResult _outhit)) (.HitBoneName (Collision|BreakHitResult _outhit)) _asbp_cowboy_character))
      (:CastFailed
        (return (.ImpactPoint (Collision|BreakHitResult _outhit)) (.PhysMat (Collision|BreakHitResult _outhit)) "" 0)))
    (else
      (return LocationEnd 0 "" 0))))