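; BP_CowboyGamemode is the game mode that reports players joining and leaving to the shooter game state.
; PostLogin passes each new player to PlayerJoined on BP_ShooterGameState, and OnLogout casts the exiting controller to PlayerController before calling PlayerLeft, printing an error if that cast fails.
; A shared GetGamestate helper casts the current game state to BP_ShooterGameState and exposes a separate CastFailed exit.
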(event EventOnLogout
  (params (ExitingController :type Controller%20Object%20Reference))
  ;[1 1 1] On Logout
  (bind _asbp_shooter_game_state (Utilities|GetGamestate)
    (:then
      (bind _asplayer_controller (Utilities|Casting|CastToPlayerController ExitingController)
        (:then
          (Default|PlayerLeft _asbp_shooter_game_state _asplayer_controller))
        (:CastFailed
          (Development|PrintString "Error in CowboyGameMode, Cast failed" true true "(R=1.000000,G=0.000000,B=0.000000,A=1.000000)"))))))

(event EventBeginPlay)

(event EventPostLogin
  (params (NewPlayer :type Player%20Controller%20Object%20Reference))
  ;[1 1 1] On Login
  (bind _asbp_shooter_game_state (Utilities|GetGamestate)
    (:then
      (Default|PlayerJoined _asbp_shooter_game_state NewPlayer))))

(fn ConstructionScript)