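; Menu game mode that hosts and joins multiplayer game sessions.
; HostGame creates a two-player LAN session and, on success, opens Level_1 as a listen server.
; JoinGame searches with LAN disabled, unlike hosting, and passes results to the Join Session graph.
; That graph joins the first result if one exists, with outcomes reported through on-screen debug prints.
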(event Custom|HostGame
  ;[1 1 1] Host Game, Create Session and Open Level_01
  (|Session (Game|GetPlayerController 0) 2 true
    (:OnSuccess
      (Game|OpenLevel(byName) "Level_1" true "listen"))))

(event Custom|JoinGame
  ;[1 1 1] Join First Game you can Find
  (bind _results (|FindSessions (Game|GetPlayerController 0) 0 false)
    (:OnSuccess
      (Utilities|JoinSession _results))
    (:OnFailure
      (Development|PrintString "No Sessiosn Available"))))

(event EventBeginPlay)

(event EventTick
  (params (DeltaSeconds :type Float%20%28single-precision%29)))

(fn ConstructionScript)